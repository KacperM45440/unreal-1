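; WaterPoints is a trigger actor that keeps a BP_Cow in play and reacts when a cow reaches its capsule.
; It spawns a cow at its SpawnPoint on BeginPlay.
; When a cow overlaps the capsule, it destroys that cow, spawns a replacement and calls JakChcesz on the top-level BP_UI widgets.
; Its own score increment and text update are disconnected and never run.
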(event `self.ReceiveBeginPlay`
  (`|SpawnActorFromClass` "/Game/Blueprints/BP_Cow.BP_Cow_C" (`KismetMathLibrary.Conv_VectorToTransform` (`SceneComponent.K2_GetComponentLocation` (`self.SpawnPoint`))) "Undefined" "MultiplyWithRoot" null null))

(event `self.Capsule.OnComponentBeginOverlap`
  (params (OverlappedComponent :type "PrimitiveComponent Object Reference") (OtherActor :type "Actor Object Reference") (OtherComp :type "PrimitiveComponent Object Reference") (OtherBodyIndex :type Integer) (bFromSweep :type Boolean) (SweepResult :type "HitResult Structure (by ref)"))
  (bind _asbp_cow (cast `/Game/Blueprints/BP_Cow` OtherActor))
  (`self.K2_DestroyActor` _asbp_cow)
  (`|SpawnActorFromClass` "/Game/Blueprints/BP_Cow.BP_Cow_C" (`KismetMathLibrary.Conv_VectorToTransform` (`SceneComponent.K2_GetComponentLocation` (`self.SpawnPoint`))) "Undefined" "MultiplyWithRoot" null null)
  (bind _foundwidgets (`WidgetBlueprintLibrary.GetAllWidgetsOfClass` "/Game/Blueprints/BP_UI.BP_UI_C"))
  (`/Game/Blueprints/BP_UI.JakChcesz` _foundwidgets))

(fn `UserConstructionScript`)